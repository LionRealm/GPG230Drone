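; Blueprint function library for the weapons system, providing helper math for targeting and lock-on.
; DecrementAndClamp lowers a value when allowed, clamps it at a minimum and flags when that floor is reached, otherwise passing it through unchanged.
; ComputeLockOnTime linearly scales lock-on time between minimum and maximum using the target's absolute stealth level as a percentage, so stealthier targets take longer to lock.
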(fn DecrementandClamp
  (params (Minimum%20Value :type Float%20%28single-precision%29) (Current%20Value :type Float%20%28single-precision%29) (Decrement%20Value :type Float%20%28single-precision%29) (Able%20To%20Decrement :type Boolean))
  (bind _returnvalue (- Current%20Value Decrement%20Value))
  (if Able%20To%20Decrement
    (LocalVariables|SetNewCurVal _returnvalue)
    (if (< Minimum%20Value _returnvalue)
      _
      (else
        (return true Minimum%20Value)))
    (else
      (LocalVariables|SetNewCurVal Current%20Value)))
  (return false (LocalVariables|GetNewCurVal)))

(fn ComputeLockonTime
  (params (TargetStruct :type Target%20Struct%20Structure) (_MaxLockonTime :type Float%20%28single-precision%29) (_MinLockonTime :type Float%20%28single-precision%29))
  (return (+ (* (Math|Float|Absolute(Float) (/ (.StealthLevel (Utilities|Struct|BreakTargetStruct TargetStruct)) 1e+02)) (- _MaxLockonTime _MinLockonTime)) _MinLockonTime)))