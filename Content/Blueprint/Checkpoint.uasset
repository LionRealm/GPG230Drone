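; Checkpoint Blueprint that registers when a FlyingPawnNewTest finishes overlapping its trigger.
; If the Pass flag is true, it broadcasts CheckpointCleared with its CheckpointNumber, hides the particle system and trigger, and disables the trigger's overlap events.
; A velocity-versus-arrow dot product for checking travel direction is present but unconnected, and this graph never sets Pass.
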(event OnComponentEndOverlap(Trigger)
  (params (OtherActor :type Actor%20Object%20Reference) (OtherComp :type Primitive%20Component%20Object%20Reference) (OtherBodyIndex :type Integer))
  ;[1 1 1] Checkpoint System
  (bind _asflying_pawn_new_test (Utilities|Casting|CastToFlyingPawnNewTest OtherActor))
  (if (Variables|Default|GetPass)
    (Default|CallCheckpointCleared (Variables|Default|GetCheckpointNumber))
    (Development|SetHiddeninGame (Variables|Default|GetParticleSystem) true false)
    (Variables|/Script/Engine.PrimitiveComponent|SetbGenerateOverlapEvents (Variables|Default|GetTrigger) false)))

(fn ConstructionScript)