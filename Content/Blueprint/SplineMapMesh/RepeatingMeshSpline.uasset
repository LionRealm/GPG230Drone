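; RepeatingMeshSpline is a construction-time actor that repeats static meshes at even intervals along a spline.
; The construction script assigns the chosen Mesh to an instanced static mesh and spaces instances by spline length over NumberOfMeshes, orienting each by spline tangent and up vector.
; A second "Top" instanced component gets a matching instance at each point, offset by a fixed distance along the base instance's up vector, so it follows banking.
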(event EventBeginPlay)

(event EventActorBeginOverlap
  (params (OtherActor :type Actor%20Object%20Reference)))

(event EventTick
  (params (DeltaSeconds :type Float%20%28single-precision%29)))

(fn ConstructionScript
  (bind _spline (Variables|Default|GetSpline))
  (bind _numberofmeshes (Variables|Default|GetNumberOfMeshes))
  (bind _instancedstaticmesh (Variables|Default|GetInstancedStaticMesh))
  (Components|StaticMesh|SetStaticMesh (Variables|Default|GetInstancedStaticMesh) (Variables|Default|GetMesh))
  (for _index (range 0 _numberofmeshes)
    (bind _returnvalue (Class|InstancedStaticMeshComponent|AddInstanceWorldSpace _instancedstaticmesh (Math|Transform|MakeTransform (Spline|GetLocationatDistanceAlongSpline _spline (* _index (/ (Spline|GetSplineLength _spline) (Math|Conversions|ToFloat(Integer) _numberofmeshes))) "World") (Math|Rotator|MakeRotfromXZ (Spline|GetTangentatDistanceAlongSpline _spline (* _index (/ (Spline|GetSplineLength _spline) (Math|Conversions|ToFloat(Integer) _numberofmeshes))) "World") (Class|SplineComponent|GetUpVectoratDistanceAlongSpline _spline (* _index (/ (Spline|GetSplineLength _spline) (Math|Conversions|ToFloat(Integer) _numberofmeshes))) "World")) "1,1,1")))
    (Class|InstancedStaticMeshComponent|AddInstanceWorldSpace (Variables|Default|GetInstancedStaticMesh%28Top%29) (Math|Transform|MakeTransform (+ (.location (.OutInstanceTransform (Components|InstancedStaticMesh|GetInstanceTransform _instancedstaticmesh _returnvalue true))) (* (Math|Vector|Normalize (Math|Vector|GetUpVector (.rotation (.OutInstanceTransform (Components|InstancedStaticMesh|GetInstanceTransform _instancedstaticmesh _returnvalue true))))) 1.9e+02)) (Math|Rotator|MakeRotfromXZ (Spline|GetTangentatDistanceAlongSpline _spline (* _index (/ (Spline|GetSplineLength _spline) (Math|Conversions|ToFloat(Integer) _numberofmeshes))) "World") (Class|SplineComponent|GetUpVectoratDistanceAlongSpline _spline (* _index (/ (Spline|GetSplineLength _spline) (Math|Conversions|ToFloat(Integer) _numberofmeshes))) "World")) "1,1,1"))))