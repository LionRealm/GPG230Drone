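; Time trial checkpoint gate that registers when a drone passes through it.
; When a drone's overlap with the trigger ends and the Pass flag is true, it broadcasts its checkpoint number, hides and disables the trigger, and plays a sound.
; A separate event recolours both gate halves through a material parameter.
; A velocity-versus-arrow direction check exists but is unconnected, and Pass is never set here.
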(event OnComponentEndOverlap(Trigger)
  (params (OtherActor :type Actor%20Object%20Reference) (OtherComp :type Primitive%20Component%20Object%20Reference) (OtherBodyIndex :type Integer))
  (bind _trigger (Variables|Default|GetTrigger))
  ;[1 1 1] Checkpoint System
  (bind _asbase_drone_class (Utilities|Casting|CastToBaseDroneClass OtherActor))
  (if (Variables|Default|GetPass)
    (Default|CallCheckpointCleared (Variables|Default|GetCheckpointNumber))
    (Development|SetHiddeninGame _trigger true false)
    (Variables|/Script/Engine.PrimitiveComponent|SetbGenerateOverlapEvents _trigger false)
    (Audio|SpawnSoundatLocation "/Game/Audio/Mastered_FX/FX_-_Checkpoint_-__-_Output_-_Stereo_Out.FX_-_Checkpoint_-__-_Output_-_Stereo_Out" (Transformation|GetWorldLocation (Variables|Default|GetRoot)))))

(event Custom|SetGateColour
  (params (NewColour :type Vector))
  ;[1 1 1] Change Gate Colour
  (Rendering|Material|SetVectorParameterValueonMaterials (Variables|Default|GetBottomHalfGate) "BaseColour" NewColour)
  (Rendering|Material|SetVectorParameterValueonMaterials (Variables|Default|GetTopHalfGate) "BaseColour" NewColour))

(fn ConstructionScript)