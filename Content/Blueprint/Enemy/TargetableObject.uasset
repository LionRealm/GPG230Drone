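; Targetable enemy object that supports missile lock-on, takes damage and respawns after a delay when its health runs out.
; Each tick it shows a heat-signature reticle only while the player's FlyingPawnWeaponsTest holds the IR Missile, sized from a computed lock-on time.
; Trace on/off functions toggle the LockOn reticle, count down lock time, resize the reticle and report when firing is allowed.
; Death hides the actor, disables collision and marks it untargetable until respawn.
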(event Custom|TargetDestroyed
  ;[1 1 1] Target Destroyed
  (Variables|General|SetHealth (Variables|General|GetMax%20Health))
  (Rendering|SetActorHiddenInGame true)
  (Collision|SetActorEnableCollision false)
  (Variables|Lockon|SetTargetInfo (Utilities|Struct|MakeTargetStruct (.TargetID (Utilities|Struct|BreakTargetStruct (Variables|Lockon|GetTargetInfo))) false (.StealthLevel (Utilities|Struct|BreakTargetStruct (Variables|Lockon|GetTargetInfo)))))
  (Utilities|FlowControl|Delay (Variables|General|GetDeath%20Duration))
  (CallFunction|TargetRespawn))

(event Custom|Target%20Respawn
  ;[1 1 1] Target Respawn
  (Rendering|SetActorHiddenInGame false)
  (Collision|SetActorEnableCollision true)
  (Variables|Lockon|SetTargetInfo (Utilities|Struct|MakeTargetStruct (.TargetID (Utilities|Struct|BreakTargetStruct (Variables|Lockon|GetTargetInfo))) true (.StealthLevel (Utilities|Struct|BreakTargetStruct (Variables|Lockon|GetTargetInfo))))))

(event EventTick
  (params (DeltaSeconds :type Float%20%28single-precision%29))
  (Utilities|FlowControl|Sequence
    (:then_0
      (bind _asflying_pawn_weapons_test (Utilities|Casting|CastToFlyingPawnWeaponsTest (Game|Player|GetPlayerPawn 0)))
      (switch Utilities|FlowControl|Switch|SwitchonWeapons (Variables|/Game/Blueprint/FlightController/Weapons/FlyingPawnWeaponsTest.FlyingPawnWeaponsTest_C|GetCurrentWeapon _asflying_pawn_weapons_test)
        (:NewEnumerator0
          (Rendering|SetVisibility (Variables|Default|GetInViewReticle) false true :!label _label))
        (:NewEnumerator1
          (Rendering|SetVisibility (Variables|Default|GetInViewReticle) true false)
          ;[1 1 1] Size Heat Signature
          (CallFunction|HeatSignatureSizer (Variables|Lockon|GetDefaultDrawSize) (Variables|Lockon|GetMaxLockonTime) (Variables|Lockon|GetMinLockonTIme) (Variables|Lockon|GetTargeted?) (Variables|Lockon|GetTargetInfo) (.targetable? (Variables|Lockon|GetTargetInfo))))
        (:NewEnumerator2
          (goto _label))
        (:NewEnumerator3
          (goto _label))))
    (:then_1
      ;[1 1 1] Check for Target Death
      (if (<= (Variables|General|GetHealth) 0.0)
        (CallFunction|TargetDestroyed)))))

(event EventBeginPlay
  ;[1 1 1] Initialize Max Health
  (Variables|General|SetHealth (Variables|General|GetMax%20Health)))

(fn ConstructionScript)

(fn AdjustReticleSize
  (params (CurrentLockonTIme :type Float%20%28single-precision%29) (MaxLockonTime :type Float%20%28single-precision%29) (TotalLockonTime :type Float%20%28single-precision%29))
  (Class|WidgetComponent|SetDrawSize (Variables|Default|GetLockOn) (* (Variables|Lockon|GetDefaultDrawSize) (+ (+ (/ CurrentLockonTIme MaxLockonTime) (/ (- MaxLockonTime TotalLockonTime) MaxLockonTime)) 0.1)))
  (return false))

(fn HeatSignatureSizer
  (params (DefaultDrawSize :type Vector%202D%20Structure) (MaxLockonTIme :type Float%20%28single-precision%29) (MinLockTime :type Float%20%28single-precision%29) (UpdateSize? :type Boolean) (TargetStruct :type Target%20Struct%20Structure) (Display? :type Boolean))
  (bind _lockontime (CallFunction|ComputeLockonTime TargetStruct MaxLockonTIme MinLockTime))
  (if UpdateSize?
    _
    (else
      (Class|WidgetComponent|SetDrawSize (Variables|Default|GetInViewReticle) (* DefaultDrawSize (+ (/ (Math|Float|Absolute(Float) (- _lockontime MaxLockonTIme)) MaxLockonTIme) 0.1)))))
  (if Display?
    (Rendering|SetVisibility (Variables|Default|GetInViewReticle) true false)
    (return false)
    (else
      (Rendering|SetVisibility (Variables|Default|GetInViewReticle) false false)
      (return false))))

(fn OnTraceOffTarget
  ;[1 1 1] Hides Reticle
  (CallFunction|ShowReticle false)
  (Variables|Lockon|SetTargeted? false)
  (return false))

(fn OnTraceOverTarget
  (params (ElapsedTime :type Float%20%28single-precision%29) (LastFrameTarget :type Target%20Struct%20Structure) (DeltaTime :type Float%20%28single-precision%29))
  (bind _targetinfo (Variables|Lockon|GetTargetInfo))
  ;[1 1 1] Initialise Local Vars
  (LocalVariables|Set_ElapsedTime ElapsedTime)
  (LocalVariables|Set_LastFrameTarget LastFrameTarget)
  (LocalVariables|Set_DeltaTime DeltaTime)
  (if (== (.TargetID (Utilities|Struct|BreakTargetStruct (LocalVariables|Get_LastFrameTarget))) (.TargetID (Utilities|Struct|BreakTargetStruct (Variables|Lockon|GetTargetInfo)))) ; Check if the same reference
    ;[1 1 1] Decrement Lock on Time
    (bind (_less_than_min _new_value) (CallFunction|DecrementandClamp 0.0 (LocalVariables|Get_ElapsedTime) (LocalVariables|Get_DeltaTime) (.Targetable? (Utilities|Struct|BreakTargetStruct (Variables|Lockon|GetTargetInfo)))))
    (CallFunction|AdjustReticleSize _new_value (Variables|Lockon|GetMaxLockonTime) (Variables|Lockon|GetTotalLockOnTime))
    (return (Variables|Lockon|GetTargetInfo) _less_than_min _new_value)
    (else
      ;[1 1 1] Compute and return info
      (bind _lockontime (CallFunction|ComputeLockonTime _targetinfo (Variables|Lockon|GetMaxLockonTime) (Variables|Lockon|GetMinLockonTIme)))
      (bind _output_get (Variables|Lockon|SetTotalLockOnTime _lockontime))
      (CallFunction|ShowReticle true)
      (Variables|Lockon|SetTargeted? true)
      (return _targetinfo false _output_get))))

(fn ShowReticle
  (params (ShowReticle? :type Boolean))
  (bind _lockon (Variables|Default|GetLockOn))
  (Rendering|SetVisibility _lockon ShowReticle? false)
  (Class|WidgetComponent|SetDrawSize _lockon (Variables|Lockon|GetDefaultDrawSize))
  (return true))

(fn TakeDamage
  (params (Damage :type Float%20%28single-precision%29))
  (bind _new_value (CallFunction|DecrementandClamp 0.0 (Variables|General|GetHealth) Damage true))
  (Variables|General|SetHealth _new_value)
  (return false))