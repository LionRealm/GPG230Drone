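; Enemy turret that locks onto and shoots the player's drone within range.
; Each Tick it checks distance, targetability and stealth, rotates toward eligible targets and recolours its material by state.
; Lock-on drives a beam, drone damage particles and a countdown, then calls PlayerShot directly with launch audio and starts a cooldown.
; Destroyed turrets turn black and clear a TargetInfo flag; construction draws a debug range sphere.
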(event EventBeginPlay
  ;[1 1 1] Init
  (|CallParentFunction)
  (Variables|ComputationVars|SetCurrentCountdown (Variables|ComputationVars|GetLockonCountdownMax))
  (bind _asmy_player_controller (Utilities|Casting|CastToMyPlayerController (Game|GetPlayerController 0))
    (:then
      (bind _output_get (Variables|PlayerVars|SetPlayerComponent _asmy_player_controller))
      (bind _asbase_drone_class (Utilities|Casting|CastToBaseDroneClass (Pawn|GetControlledPawn _output_get)))
      (Variables|Default|SetPlayerPawn _asbase_drone_class)
      (bind _returnvalue (Effects|SpawnEmitterAttached "/Game/Particles/P_Beam.P_Beam" (Variables|Default|GetFirePoint) "None"))
      (Variables|Default|SetLazerParticle _returnvalue))
    (:CastFailed
      (Development|PrintString "Could not cast to My Player Controller"))))

(event EventTick
  (params (DeltaSeconds :type Float%20%28single-precision%29))
  (bind _returnvalue (Utilities|Time|GetWorldDeltaSeconds))
  (bind _turret_lowpoly (Variables|Default|GetTurret_LowPoly))
  (bind _playercomponent (Variables|PlayerVars|GetPlayerComponent))
  (bind _returnvalue_2 (Transformation|GetWorldRotation _turret_lowpoly))
  (bind _returnvalue_3 (Transformation|GetWorldLocation _turret_lowpoly))
  (bind _returnvalue_4 (Pawn|GetControlledPawn _playercomponent))
  (bind _returnvalue_5 (Transformation|GetActorLocation _returnvalue_4))
  (bind _returnvalue_6 (Math|Rotator|FindLookatRotation _returnvalue_3 _returnvalue_5))
  (bind _returnvalue_7 (+ (.yaw _returnvalue_6) -9e+01))
  (bind _returnvalue_8 (Math|Interpolation|RInterpTo _returnvalue_2 (Math|Rotator|MakeRotator (.roll _returnvalue_6) (.pitch _returnvalue_6) _returnvalue_7) _returnvalue 1e+01))
  (|CallParentFunction DeltaSeconds)
  (if (Variables|Default|GetDestroyed?)
    ;[1 1 1] Set Colour to Black
    (Rendering|Material|SetVectorParameterValueonMaterials (Variables|Default|GetTurret_LowPoly) "TurretColour" "0.000000,0.000000,0.000000")
    (Variables|Default|SetTargetInfo (Utilities|Struct|MakeTargetStruct (.targetid (Variables|Default|GetTargetInfo)) false (.stealthlevel (Variables|Default|GetTargetInfo))))
    (else
      (CallFunction|DecrementFireCooldown)
      (if (>= (Transformation|GetDistanceTo self _returnvalue_4) (Variables|EnemyVars|GetDistanceTillLockon))
        ;[1 1 1] Set Colour to Grey
        (Rendering|Material|SetVectorParameterValueonMaterials (Variables|Default|GetTurret_LowPoly) "TurretColour" "0.200000,0.200000,0.200000" :!label _label)
        (bind _asbase_drone_class (Utilities|Casting|CastToBaseDroneClass (Pawn|GetControlledPawn (Variables|PlayerVars|GetPlayerComponent)) :!label _label_2))
        (Default|PlayerLockedonto _asbase_drone_class false)
        ;[1 1 1] Clear Beam Target
        (Class|ParticleSystemComponent|SetBeamTargetPoint (Variables|Default|GetLazerParticle) 0 (Transformation|GetWorldLocation (Variables|Default|GetFirePoint)))
        (for _array_element (Variables|/Game/Blueprint/FlightController/Base/BaseDroneClass.BaseDroneClass_C|GetDamageParticleEffect _asbase_drone_class)
          (Rendering|SetVisibility _array_element false false)
          (CallFunction|ResetCountdown))
        (else
          (bind _asbase_drone_class_2 (Utilities|Casting|CastToBaseDroneClass (Pawn|GetControlledPawn (Variables|PlayerVars|GetPlayerComponent))))
          (if (.targetable? (Variables|/Game/Blueprint/FlightController/Base/BaseDroneClass.BaseDroneClass_C|GetPlayerTarget%20Stats _asbase_drone_class_2))
            ;[1 1 1] Set Turret to rotate towards player
            (Transformation|SetWorldRotation (Variables|Default|GetTurret_LowPoly) (Math|Rotator|MakeRotator 0.0 (Math|Float|ClampAngle (.pitch _returnvalue_8) -1e+02 1.7e+02) (.yaw _returnvalue_8)) false false)
            ;[1 1 1] Check stealth level
            (bind _asbase_drone_class_3 (Utilities|Casting|CastToBaseDroneClass _returnvalue_4)
              (:then
                (if (< (Variables|EnemyVars|GetPlayerStealthThreshold) (.stealthlevel (Variables|/Game/Blueprint/FlightController/Base/BaseDroneClass.BaseDroneClass_C|GetPlayerTarget%20Stats _asbase_drone_class_3)))
                  ;[1 1 1] Set turret colour orange
                  (Rendering|Material|SetVectorParameterValueonMaterials (Variables|Default|GetTurret_LowPoly) "TurretColour" "1.000000,0.800000, 0")
                  (goto _label_2)
                  (else
                    ;[1 1 1] Set turret colour red
                    (Rendering|Material|SetVectorParameterValueonMaterials (Variables|Default|GetTurret_LowPoly) "TurretColour" "1.000000,0.000000,0.000000")
                    (Utilities|FlowControl|Sequence
                      (:then_0
                        (bind _asbase_drone_class_4 (Utilities|Casting|CastToBaseDroneClass (Pawn|GetControlledPawn (Variables|PlayerVars|GetPlayerComponent))))
                        (Default|PlayerLockedonto _asbase_drone_class_4 true))
                      (:then_1
                        ;[1 1 1] Countdown
                        (Variables|ComputationVars|SetCurrentCountdown (- (Variables|ComputationVars|GetCurrentCountdown) (Utilities|Time|GetWorldDeltaSeconds)))
                        ;[1 1 1] Is Countdown less than 0?
                        (if (< (Variables|ComputationVars|GetCurrentCountdown) 0.0)
                          ;[1 1 1] Is able to fire?
                          (if (Variables|ComputationVars|GetCanFire?)
                            ;[1 1 1] Fire Missile
                            (bind _asbase_drone_class_5 (Utilities|Casting|CastToBaseDroneClass (Pawn|GetControlledPawn (Variables|PlayerVars|GetPlayerComponent))))
                            (Default|PlayerShot _asbase_drone_class_5)
                            (Variables|ComputationVars|SetCurrentCountdown (Variables|ComputationVars|GetLockonCountdownMax))
                            (Variables|ComputationVars|SetCanFire? false)
                            (Variables|ComputationVars|SetCurrentFireCooldown (Variables|EnemyVars|GetAfterFireCooldown))
                            (Audio|SpawnSoundAttached "/Game/Audio/Fx_-_Missile_Launch.Fx_-_Missile_Launch" 0))))
                      (:then_2
                        ;[1 1 1] Set Beam Target
                        (bind _asbase_drone_class_6 (Utilities|Casting|CastToBaseDroneClass (Pawn|GetControlledPawn (Variables|PlayerVars|GetPlayerComponent))))
                        (Class|ParticleSystemComponent|SetBeamTargetPoint (Variables|Default|GetLazerParticle) 0 (Transformation|GetWorldLocation (Variables|/Game/Blueprint/FlightController/Base/BaseDroneClass.BaseDroneClass_C|GetLazerPoint _asbase_drone_class_6)))
                        (for _array_element_2 (Variables|/Game/Blueprint/FlightController/Base/BaseDroneClass.BaseDroneClass_C|GetDamageParticleEffect _asbase_drone_class_6)
                          (if (not (Rendering|IsVisible _array_element_2))
                            (Rendering|SetVisibility _array_element_2 true false))))))))
              (:CastFailed
                ;[1 1 1] Error
                (Development|PrintString "Error, Could not cast to correct pawn")))
            (else
              (goto _label))))))))

(fn ConstructionScript
  (|CallParentFunction)
  (Rendering|Debug|DrawDebugSphere (Transformation|GetWorldLocation (Variables|Default|GetRoot)) (Variables|EnemyVars|GetDistanceTillLockon) 12 "(R=0.615000,G=0.004698,B=0.000000,A=1.000000)" 5.0))

(fn ResetCountdown
  (Variables|ComputationVars|SetCurrentCountdown (Variables|ComputationVars|GetLockonCountdownMax))
  (return))

(fn DecrementFireCooldown
  ;[1 1 1] Decrement Can Fire
  (if (Variables|ComputationVars|GetCanFire?)
    _
    (else
      (Variables|ComputationVars|SetCurrentFireCooldown (- (Variables|ComputationVars|GetCurrentFireCooldown) (Utilities|Time|GetWorldDeltaSeconds)))
      (if (>= 0.0 (Variables|ComputationVars|GetCurrentFireCooldown))
        (Variables|ComputationVars|SetCanFire? true))))
  (return))

(fn GetDistancetoPlayer
  (return (>= (Transformation|GetDistanceTo self (Pawn|GetControlledPawn (Variables|PlayerVars|GetPlayerComponent))) (Variables|EnemyVars|GetDistanceTillLockon))))