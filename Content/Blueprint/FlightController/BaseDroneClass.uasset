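; Base player-flown drone with arcade flight controls, lock-on warning beep and crash respawn.
; Axis inputs set clamped speed and interpolated pitch and yaw rates, which Tick applies to PlaneMesh with pitch limits and yaw-driven banking.
; Throttle and brakes also write an inverse speed percentage into PlayerTargetStats.
; Any hit hides the drone and destroys it after a delay, then MyPlayerController respawns it, having stored the start transform at BeginPlay.
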(event Custom|PlayerLockedOnTo
  (params (LockOnState :type Boolean))
  ;[1 1 1] LockOnBeep
  (bind _output_get (Variables|PlayerStats|SetLockedOn LockOnState))
  (if _output_get
    (Audio|SpawnSoundAttached "/Game/Audio/Fx_-_Lock_On_Beep.Fx_-_Lock_On_Beep" (Variables|Default|GetCamera) "None" "0, 0, 0" "0, 0, 0" "KeepRelativeOffset" true 0.3)))

(event EventTick
  (params (DeltaSeconds :type Float%20%28single-precision%29))
  (bind _plane_mesh (Variables|Default|GetPlane%20mesh))
  (bind _plane_mesh_2 (Variables|Default|GetPlane%20mesh))
  (bind _current_forward_speed (Variables|CalculationVars|GetCurrent%20forward%20speed))
  (bind _plane_mesh_3 (Variables|Default|GetPlane%20mesh))
  (bind _returnvalue (Math|Vector|GetForwardVector _plane_mesh))
  (bind _returnvalue_2 (* DeltaSeconds _current_forward_speed))
  (bind _relativerotation (Variables|/Script/Engine.SceneComponent|GetRelativeRotation _plane_mesh_2))
  (bind _relativerotation_2 (Variables|/Script/Engine.SceneComponent|GetRelativeRotation _plane_mesh_3))
  ;[1 1 1] Init / Forward Movement
  (Utilities|FlowControl|Sequence
    (:then_1
      (Transformation|AddWorldOffset (Variables|Default|GetPlane%20mesh) (Math|Vector|MakeVector (* _returnvalue_2 (.x _returnvalue)) (* _returnvalue_2 (.y _returnvalue)) (* _returnvalue_2 (.z _returnvalue))) true false)
      (Transformation|AddWorldRotation (Variables|Default|GetPlane%20mesh) (Math|Rotator|MakeRotator 0.0 0.0 (* (Utilities|Time|GetWorldDeltaSeconds) (Variables|CalculationVars|GetCurrent%20yaw%20speed))) true false)
      (Transformation|AddRelativeRotation (Variables|Default|GetPlane%20mesh) (Math|Rotator|MakeRotator 0.0 (* (Utilities|Time|GetWorldDeltaSeconds) (Variables|CalculationVars|GetCurrent%20pitch%20speed)) 0.0) true false)
      (Transformation|SetRelativeRotation (Variables|Default|GetPlane%20mesh) (Math|Rotator|MakeRotator (.roll _relativerotation_2) (Math|Float|Clamp(Float) (.pitch _relativerotation_2) (Variables|FlightVars|GetMin%20Pitch) (Variables|FlightVars|GetMax%20Pitch)) (.yaw _relativerotation_2)) true false)
      (Transformation|SetRelativeRotation (Variables|Default|GetPlane%20mesh) (Math|Rotator|MakeRotator (* (Variables|FlightVars|GetRoll%20Multiplier) (* (Utilities|Time|GetWorldDeltaSeconds) (Variables|CalculationVars|GetCurrent%20yaw%20speed))) (.pitch _relativerotation) (.yaw _relativerotation)) true false))))

(event Collision|EventHit
  (params (MyComp :type Primitive%20Component%20Object%20Reference) (Other :type Actor%20Object%20Reference) (OtherComp :type Primitive%20Component%20Object%20Reference) (bSelfMoved :type Boolean) (HitLocation :type Vector :default "0, 0, 0") (HitNormal :type Vector) (NormalImpulse :type Vector :default "0, 0, 0") (Hit :type Hit%20Result%20Structure%20%28by%20ref%29))
  ;[1 1 1] Deflect when colliding
  (Development|PrintString "HIT")
  (Transformation|SetActorRotation (Math|Rotator|Lerp(Rotator) (Transformation|GetActorRotation) (Math|Conversions|RotationFromXVector HitNormal) 0.025 true))
  (Rendering|SetActorHiddenInGame true)
  (Actor|Tick|SetActorTickEnabled false)
  (Utilities|FlowControl|Delay 2.0)
  (Variables|CalculationVars|SetCrashed true)
  (Actor|DestroyActor))

(event EventBeginPlay
  (bind _asmy_player_controller (Utilities|Casting|CastToMyPlayerController (Game|GetPlayerController 0)))
  (bind _output_get (Variables|General|SetController%20Reference _asmy_player_controller))
  (Variables|/Game/Blueprint/MyPlayerController.MyPlayerController_C|SetRespawnLocation _output_get (Transformation|GetActorTransform)))

(event EventDestroyed
  (if (Variables|CalculationVars|GetCrashed)
    (Default|RespawnVehicle (Variables|General|GetController%20Reference))))

(event Input|AxisEvents|InputAxisBrakes
  (params (AxisValue :type Float%20%28single-precision%29))
  (bind _maxspeed (Variables|FlightVars|GetMaxSpeed))
  (bind _min_speed (Variables|FlightVars|GetMin%20speed))
  ;[1 1 1] Deceleration
  (Variables|PlayerStats|SetPlayerTarget%20Stats (Utilities|Struct|MakeTargetStruct (.targetid (Variables|PlayerStats|GetPlayerTarget%20Stats)) (.targetable? (Variables|PlayerStats|GetPlayerTarget%20Stats)) (Math|Float|Absolute(Float) (* (- (Math|Float|NormalizetoRange (Math|Float|Clamp(Float) (+ (Variables|CalculationVars|GetCurrent%20forward%20speed) (* (* AxisValue (Variables|FlightVars|GetAcceleration)) (Utilities|Time|GetWorldDeltaSeconds))) _min_speed _maxspeed) _min_speed _maxspeed) 1.0) 1e+02))))
  (Variables|CalculationVars|SetCurrent%20forward%20speed (Math|Float|Clamp(Float) (+ (Variables|CalculationVars|GetCurrent%20forward%20speed) (* (* AxisValue (Variables|FlightVars|GetAcceleration)) (Utilities|Time|GetWorldDeltaSeconds))) _min_speed _maxspeed)) ; Update forward speed based on input axis value
)

(event Input|AxisEvents|InputAxisMoveUp
  (params (AxisValue :type Float%20%28single-precision%29))
  ;[1 1 1] Up/Down
  (Variables|CalculationVars|SetCurrent%20pitch%20speed (Math|Interpolation|FInterpTo (Variables|CalculationVars|GetCurrent%20pitch%20speed) (* AxisValue 25.0 -1.0) (Utilities|Time|GetWorldDeltaSeconds) 2.0)))

(event Input|AxisEvents|InputAxisThrust
  (params (AxisValue :type Float%20%28single-precision%29))
  (bind _maxspeed (Variables|FlightVars|GetMaxSpeed))
  (bind _min_speed (Variables|FlightVars|GetMin%20speed))
  ;[1 1 1] Thrust
  (Variables|PlayerStats|SetPlayerTarget%20Stats (Utilities|Struct|MakeTargetStruct (.targetid (Variables|PlayerStats|GetPlayerTarget%20Stats)) (.targetable? (Variables|PlayerStats|GetPlayerTarget%20Stats)) (Math|Float|Absolute(Float) (* (- (Math|Float|NormalizetoRange (Math|Float|Clamp(Float) (+ (Variables|CalculationVars|GetCurrent%20forward%20speed) (* (* AxisValue (Variables|FlightVars|GetAcceleration)) (Utilities|Time|GetWorldDeltaSeconds))) _min_speed _maxspeed) _min_speed _maxspeed) 1.0) 1e+02))))
  (Variables|CalculationVars|SetCurrent%20forward%20speed (Math|Float|Clamp(Float) (+ (Variables|CalculationVars|GetCurrent%20forward%20speed) (* (* AxisValue (Variables|FlightVars|GetAcceleration)) (Utilities|Time|GetWorldDeltaSeconds))) _min_speed _maxspeed)) ; Update forward speed based on input axis value
)

(event Input|AxisEvents|InputAxisMoveRight
  (params (AxisValue :type Float%20%28single-precision%29))
  ;[1 1 1] Turning
  (Variables|CalculationVars|SetCurrent%20yaw%20speed (Math|Interpolation|FInterpTo (Variables|CalculationVars|GetCurrent%20yaw%20speed) (* AxisValue (Variables|FlightVars|GetTurn%20speed)) (Utilities|Time|GetWorldDeltaSeconds) 2.0)))

(fn ConstructionScript)

(fn RespawnCheck)