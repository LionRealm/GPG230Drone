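; Spline actor that repeats a chosen static mesh at even intervals along its path, apparently for track building.
; The construction script clears and rebuilds an instanced static mesh component, dividing spline length by NumberOfMeshes to space instances.
; Each instance takes the spline's world location and rotation at that distance, at unit scale.
; Disconnected leftovers include a second, up-offset instance and alternative rotation math; the event graph is empty.
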(event EventBeginPlay)

(event EventActorBeginOverlap
  (params (OtherActor :type Actor%20Object%20Reference)))

(event EventTick
  (params (DeltaSeconds :type Float%20%28single-precision%29)))

(fn ConstructionScript
  (bind _spline (Variables|Default|GetSpline))
  (bind _numberofmeshes (Variables|Default|GetNumberOfMeshes))
  (bind _instancedstaticmesh (Variables|Default|GetInstancedStaticMesh))
  (Components|StaticMesh|SetStaticMesh _instancedstaticmesh (Variables|Default|GetMesh))
  (Components|InstancedStaticMesh|ClearInstances _instancedstaticmesh)
  (for _index (range 0 _numberofmeshes)
    (bind _returnvalue (Class|InstancedStaticMeshComponent|AddInstanceWorldSpace (Variables|Default|GetInstancedStaticMesh) (Math|Transform|MakeTransform (Spline|GetLocationatDistanceAlongSpline _spline (* _index (/ (Spline|GetSplineLength _spline) (Math|Conversions|ToFloat(Integer) _numberofmeshes))) "World") (Spline|GetRotationatDistanceAlongSpline _spline (* _index (/ (Spline|GetSplineLength _spline) (Math|Conversions|ToFloat(Integer) _numberofmeshes))) "World") "1,1,1")))))