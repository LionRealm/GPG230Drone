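; TargetInterface is an interface in the TestWeapons folder for objects that weapons can trace, lock on to and damage.
; It declares trace-over and trace-off events, with trace-over taking elapsed time and the last-frame target and returning a can-fire flag and updated time.
; Other functions cover showing and resizing the reticle from lock-on times, sizing a heat signature display, and taking damage.
; All graphs are signatures without logic.
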(fn OnTraceOverTarget
  (params (ElapsedTime :type Float%20%28single-precision%29) (LastFrameTarget :type Target%20Struct%20Structure) (DeltaTime :type Float%20%28single-precision%29))
  (return "" false 0.0))

(fn OnTraceOffTarget
  (return false))

(fn ShowReticle
  (return false))

(fn AdjustReticleSize
  (params (CurrentLockonTIme :type Float%20%28single-precision%29) (MaxLockonTime :type Float%20%28single-precision%29) (TotalLockonTime :type Float%20%28single-precision%29))
  (return false))

(fn HeatSignatureSizer
  (params (DefaultDrawSize :type Vector%202D%20Structure) (MaxLockonTIme :type Float%20%28single-precision%29) (MinLockTime :type Float%20%28single-precision%29) (UpdateSize? :type Boolean) (TargetStruct :type Target%20Struct%20Structure) (Display? :type Boolean))
  (return false))

(fn TakeDamage
  (params (Damage :type Float%20%28single-precision%29))
  (return false))