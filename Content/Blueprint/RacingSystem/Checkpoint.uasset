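; Racing checkpoint gate that signals when a FlyingPawnWeaponsTest pawn leaves its trigger.
; If Pass is true, end overlap broadcasts the checkpoint number through CheckpointCleared, hides the trigger, disables its overlaps and plays a sound at the root.
; SetGateColour recolours both gate halves through their BaseColour material parameter.
; A velocity-versus-arrow direction check is present but unused, and nothing here sets Pass.
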(event OnComponentEndOverlap(Trigger)
  (params (OtherActor :type Actor%20Object%20Reference) (OtherComp :type Primitive%20Component%20Object%20Reference) (OtherBodyIndex :type Integer))
  (bind _trigger (Variables|Default|GetTrigger))
  ;[1 1 1] Checkpoint System
  (bind _asflying_pawn_weapons_test (Utilities|Casting|CastToFlyingPawnWeaponsTest OtherActor))
  (if (Variables|Default|GetPass)
    (Default|CallCheckpointCleared (Variables|Default|GetCheckpointNumber))
    (Development|SetHiddeninGame _trigger true false)
    (Variables|/Script/Engine.PrimitiveComponent|SetbGenerateOverlapEvents _trigger false)
    (Audio|SpawnSoundatLocation "/Game/Audio/Fx_-_Checkpoint.Fx_-_Checkpoint" (Transformation|GetWorldLocation (Variables|Default|GetRoot)))))

(event Custom|SetGateColour
  (params (NewColour :type Vector))
  ;[1 1 1] Change Gate Colour
  (Rendering|Material|SetVectorParameterValueonMaterials (Variables|Default|GetBottomHalfGate) "BaseColour" NewColour)
  (Rendering|Material|SetVectorParameterValueonMaterials (Variables|Default|GetTopHalfGate) "BaseColour" NewColour))

(fn ConstructionScript)